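; A player character Blueprint that drives a building system through a UI widget and mouse input.
; BeginPlay creates the hidden build widget and caches references to the BP_Car and BP_Car2 actors in the level.
; Tab flip-flops the widget and mouse cursor, clearing the building component's selected mesh class on opening, while Click calls that component's Move function.
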(event `self.ReceiveBeginPlay`
  (bind _returnvalue (`|CreateWidget` "/Game/Dev/JJH/WB_BuildSystemWidget.WB_BuildSystemWidget_C"))
  (bind _output_get (set `self.WB_Widget` _returnvalue))
  (`UserWidget.AddToViewport` _output_get 0)
  (`Widget.SetVisibility` _output_get "Hidden")
  (bind _returnvalue_2 (`GameplayStatics.GetActorOfClass` "/Game/Dev/JJH/BP_Car.BP_Car_C"))
  (set `self.car1` _returnvalue_2)
  (bind _returnvalue_3 (`GameplayStatics.GetActorOfClass` "/Game/Dev/JJH/BP_Car2.BP_Car2_C"))
  (set `self.car2` _returnvalue_3))

(event `InputAction|Tab key`
  (params (Key :type "Key Structure"))
  (:`Pressed`
    (`/Engine/EditorBlueprintResources/StandardMacros.FlipFlop`
      (:`A`
        (set `/Game/Dev/JJH/ACBP_BuildingSystem.meshclass` null (`self.ACBP_BuildingSystem`))
        (set `PlayerController.bShowMouseCursor` true (`GameplayStatics.GetPlayerController` 0))
        (`Widget.SetVisibility` (`self.WB_Widget`) "Visible"))
      (:`B`
        (set `PlayerController.bShowMouseCursor` false (`GameplayStatics.GetPlayerController` 0))
        (`Widget.SetVisibility` (`self.WB_Widget`) "Hidden")))))

(event `InputAction|Click`
  (params (Key :type "Key Structure"))
  (:`Pressed`
    (`/Game/Dev/JJH/ACBP_BuildingSystem.move` (`self.ACBP_BuildingSystem`))))

(fn `UserConstructionScript`)