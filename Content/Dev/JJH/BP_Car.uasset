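; BP_Car is a placeable car actor for the VR building system, with a swappable SpawnMesh.
; Mesh overlap events set the player widget's Isoverlap flag and, while this actor is the building system's spawned mesh, switch it between two preview materials.
; The build event sets materials from the build widget's selection flags, using a clean material, one read from a BP_Car2 in the level, or other slot-zero overrides.
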(event `self.ReceiveBeginPlay`)

(event `setMesh`
  (`StaticMeshComponent.SetStaticMesh` (`self.SpawnMesh`) (`self.MeshChange`)))

(event `build`
  (bind _wb_widget (`self.WB Widget`))
  (bind _returnvalue (`MeshComponent.GetMaterialIndex` (`self.SpawnMesh`) "None"))
  (bind _aswb_build_system_widget (cast `/Game/Dev/JJH/WB_BuildSystemWidget` _))
  (set `self.WB Widget` _aswb_build_system_widget)
  (bind _isselect1 (`/Game/Dev/JJH/WB_BuildSystemWidget.isselect1` _aswb_build_system_widget))
  (`KismetSystemLibrary.PrintString` (`KismetStringLibrary.Conv_BoolToString` _isselect1))
  (if _isselect1
    (for (_ _array_index) (`|MakeArray` _returnvalue _returnvalue _returnvalue _returnvalue _returnvalue _returnvalue _returnvalue)
      (`PrimitiveComponent.SetMaterial` (`self.SpawnMesh`) _array_index "/Game/LMH/cleanMat.cleanMat")
      (`KismetSystemLibrary.PrintString` "222"))
    (elif (`/Game/Dev/JJH/WB_BuildSystemWidget.isselect2` (`self.WB Widget`))
      (bind _returnvalue_2 (`GameplayStatics.GetActorOfClass` "/Game/Dev/JJH/BP_Car2.BP_Car2_C"))
      (bind _sm_sedan_01a (`/Game/Dev/JJH/BP_Car2.SM_Sedan_01a` _returnvalue_2))
      (bind _returnvalue_3 (`MeshComponent.GetMaterialIndex` _sm_sedan_01a "None"))
      (for (_ _array_index_2) (`|MakeArray` _returnvalue_3 _returnvalue_3 _returnvalue_3 _returnvalue_3 _returnvalue_3 _returnvalue_3 _returnvalue_3)
        (`PrimitiveComponent.SetMaterial` (`self.SpawnMesh`) _array_index_2 (`PrimitiveComponent.GetMaterial` _sm_sedan_01a _returnvalue_3)))
      (elif (`/Game/Dev/JJH/WB_BuildSystemWidget.isselect3` _wb_widget)
        (`PrimitiveComponent.SetMaterial` (`self.SpawnMesh`) 0 null)
        (elif (`/Game/Dev/JJH/WB_BuildSystemWidget.isselect4` _wb_widget)
          (`PrimitiveComponent.SetMaterial` (`self.SpawnMesh`) 0 "/Game/StarterContent/Props/Materials/M_Chair.M_Chair"))))))

(event `self.SpawnMesh.OnComponentEndOverlap`
  (params (OverlappedComponent :type "PrimitiveComponent Object Reference") (OtherActor :type "Actor Object Reference") (OtherComp :type "PrimitiveComponent Object Reference") (OtherBodyIndex :type Integer))
  (bind _returnvalue (`MeshComponent.GetMaterialIndex` (`self.SpawnMesh`) "None"))
  (bind _asbp_vrcharacter (cast `/Game/LSH_WorkSpace/BP_VRCharacter` (`GameplayStatics.GetPlayerCharacter` 0)))
  (set `/Game/Dev/JJH/WB_BuildSystemWidget.isoverlap` false (`/Game/LSH_WorkSpace/BP_VRCharacter.WB_Widget` _asbp_vrcharacter))
  (if (== (`/Game/Dev/JJH/ACBP_BuildingSystem.Spawnedmesh` (`/Game/LSH_WorkSpace/BP_VRCharacter.ACBP_BuildingSystem` _asbp_vrcharacter)) self)
    (for (_ _array_index) (`|MakeArray` _returnvalue _returnvalue _returnvalue _returnvalue _returnvalue _returnvalue _returnvalue)
      (`PrimitiveComponent.SetMaterial` (`self.SpawnMesh`) _array_index "/Game/Dev/JJH/M_green.M_green"))))

(event `move`)

(event `self.SpawnMesh.OnComponentBeginOverlap`
  (params (OverlappedComponent :type "PrimitiveComponent Object Reference") (OtherActor :type "Actor Object Reference") (OtherComp :type "PrimitiveComponent Object Reference") (OtherBodyIndex :type Integer) (bFromSweep :type Boolean) (SweepResult :type "HitResult Structure (by ref)"))
  (bind _returnvalue (`MeshComponent.GetMaterialIndex` (`self.SpawnMesh`) "None"))
  (bind _asbp_vrcharacter (cast `/Game/LSH_WorkSpace/BP_VRCharacter` (`GameplayStatics.GetPlayerCharacter` 0)))
  (set `/Game/Dev/JJH/WB_BuildSystemWidget.isoverlap` true (`/Game/LSH_WorkSpace/BP_VRCharacter.WB_Widget` _asbp_vrcharacter))
  (if (== (`/Game/Dev/JJH/ACBP_BuildingSystem.Spawnedmesh` (`/Game/LSH_WorkSpace/BP_VRCharacter.ACBP_BuildingSystem` _asbp_vrcharacter)) self)
    (for (_ _array_index) (`|MakeArray` _returnvalue _returnvalue _returnvalue _returnvalue _returnvalue _returnvalue _returnvalue)
      (`PrimitiveComponent.SetMaterial` (`self.SpawnMesh`) _array_index "/Game/Dev/JJH/M_green_2.M_green_2"))))

(fn `UserConstructionScript`)