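; BP_Splashes is a water splash effect Blueprint that drives a Niagara system with configurable mesh, material and spawn settings.
; On construction it picks a mesh by vertex detail and splash type, creates a dynamic material from it, and passes both plus spawn parameters to Niagara.
; BeginPlay hands Niagara a self reference and Performance value.
; When RunInSequencer is set, Tick reapplies material and spawn parameters for cinematic animation.
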(event `self.ReceiveTick`
  (params (DeltaSeconds :type "Float (single-precision)"))
  (bind _apply_sp_material (`self.Apply_SP_Material`))
  (bind _niagara (`self.Niagara`))
  (bind _niagara_2 (`self.Niagara`))
  ;[1 0 0 1 110] Change parameters in Cinematic Mode
  (if (`self.RunInSequencer`)
    (`/Engine/EditorBlueprintResources/StandardMacros.IsValid` _apply_sp_material
      (:`Is Valid`
        (`MaterialInstanceDynamic.SetVectorParameterValue` _apply_sp_material "Color" (`self.Color`))
        (`MaterialInstanceDynamic.SetScalarParameterValue` _apply_sp_material "Opacity" (`self.Opacity`))
        (`MaterialInstanceDynamic.SetScalarParameterValue` _apply_sp_material "InIQR" (`self.InIOR`))
        (`MaterialInstanceDynamic.SetScalarParameterValue` _apply_sp_material "OutIQR" (`self.OutIOR`))
        (`MaterialInstanceDynamic.SetScalarParameterValue` _apply_sp_material "Metalic" (`self.Metalic`))
        (`MaterialInstanceDynamic.SetScalarParameterValue` _apply_sp_material "Emessive" (`self.Emissive`))
        (`MaterialInstanceDynamic.SetScalarParameterValue` _apply_sp_material "Spacular" (`self.Spacular`))
        (`MaterialInstanceDynamic.SetScalarParameterValue` _apply_sp_material "Rouphness" (`self.Rouphness`))
        (`MaterialInstanceDynamic.SetScalarParameterValue` _apply_sp_material "MultyVelocity" (`self.Foam_Multy_Splash`))
        (`MaterialInstanceDynamic.SetScalarParameterValue` _apply_sp_material "PowerVelocity" (`self.Foam_Power_Splash`))
        (`|ExecutionSequence`
          (:`then_0`
            (`NiagaraComponent.SetVariableFloat` _niagara "Splash_Spawn Rate" (`self.Splash_Spawn Rate`))
            (`NiagaraComponent.SetVariableFloat` _niagara "HML_OutMaxFrame" (`self.HML_FramOut`)))
          (:`then_1`
            (`NiagaraComponent.SetVariableFloat` _niagara_2 "SplashScale" (`self.SplashScale`))
            (`NiagaraComponent.SetVariableFloat` _niagara_2 "SplashTime" (`self.SplashLifeTime`))))))))

(event `self.ReceiveBeginPlay`
  (bind _niagara (`self.Niagara`))
  ;[1 1 1 1 100] Add Blueprint to Niagara Object variable
  (`NiagaraComponent.SetVariableObject` _niagara "BP" self)
  (`NiagaraComponent.SetVariableFloat` _niagara "Performance" (`KismetMathLibrary.MapRangeClamped` 0.0 0.0 1.0 0.1 10.0)))

(fn `UserConstructionScript`
  (`self.SetUpParameters`))