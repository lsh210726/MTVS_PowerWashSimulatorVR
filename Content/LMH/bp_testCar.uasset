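; Test car actor that can be painted by aiming the player camera at its mesh.
; Each Tick it line-traces the mesh along the camera's forward vector and passes hits to the VR character's DrawComp.DrawCar.
; DrawOnWhiteBoard stamps a dynamic brush material into the PaintBoard render target at a given location, and DrawSize sets brush size.
; Board-switch binding, target clearing and material-swap nodes are left disconnected.
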(event `self.ReceiveTick`
  (params (DeltaSeconds :type "Float (single-precision)"))
  (bind _transformcomponent (`PlayerCameraManager.TransformComponent` (`GameplayStatics.GetPlayerCameraManager` 0)))
  (bind _returnvalue (`SceneComponent.K2_GetComponentLocation` _transformcomponent))
  ;[0 0.3539 1] Ray from CameraManager
  (bind (_hitlocation _hitnormal _bonename _outhit _returnvalue_2) (`PrimitiveComponent.K2_LineTraceComponent` (`self.StaticMesh`) _returnvalue (+ _returnvalue (* (`SceneComponent.GetForwardVector` _transformcomponent) 10000.0)) true true false))
  (if _returnvalue_2
    ;[1 1 1] Find world position for 3d brush on a surface of the painted object
    (bind _asbp_vrcharacter (cast `/Game/LSH_WorkSpace/BP_VRCharacter` (`GameplayStatics.GetPlayerPawn` 0)))
    (`RenderTargetProcess.DrawCar` (`VRCharacter.DrawComp` _asbp_vrcharacter) _outhit)))

(event `BoardChange_Event_0`
  (set `self.PaintBoard` "/Game/LMH/protomap/2PaintBoard.2PaintBoard"))

(event `self.ReceiveBeginPlay`
  (`|ExecutionSequence`
    (:`then_0`
      (bind _returnvalue (`KismetMaterialLibrary.CreateDynamicMaterialInstance` "/Game/LMH/protomap/WhiteBoardMarker.WhiteBoardMarker"))
      (set `self.WhiteBoardMarker` _returnvalue))
    (:`then_1`
      (set `self.PaintBoard` "/Game/LMH/protomap/1PaintBoard.1PaintBoard"))))

(event `DrawOnWhiteBoard`
  (params (`Location to Draw` :type "Vector2D Structure"))
  (bind _whiteboardmarker (`self.WhiteBoardMarker`))
  (`MaterialInstanceDynamic.SetVectorParameterValue` _whiteboardmarker "DrawLocation" (`KismetMathLibrary.Conv_VectorToLinearColor` (`KismetMathLibrary.Conv_Vector2DToVector` `Location to Draw` 0.1)))
  ;[1 1 1] target 에 mat그림
  (`KismetRenderingLibrary.DrawMaterialToRenderTarget` (`self.PaintBoard`) _whiteboardmarker))

(event `DrawSize`
  (params (`Draw Size` :type "Float (double-precision)"))
  (`MaterialInstanceDynamic.SetScalarParameterValue` (`self.WhiteBoardMarker`) "Size" `Draw Size`))

(fn `UserConstructionScript`)