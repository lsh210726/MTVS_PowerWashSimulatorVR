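; Box truck actor that generates dirt stains when triggered through the VR player character.
; On BeginPlay it binds its createdirty event to BP_VRCharacter's Createdirty dispatcher.
; That event has DirtyStain create stains from the Ray3 child actor's location using a multi-trace cone.
; Overlap, build and move events are empty, and the material-swap, collision and decal logic is disconnected.
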(event `createdirty_Event`
  (`DirtyStainComponent.CreateDirtyStatin` (`self.DirtyStain`) (`self.K2_GetActorLocation` (`ChildActorComponent.ChildActor` (`self.ray3`))) 1000.0 10 60.0))

(event `self.ReceiveBeginPlay`
  (bind _asbp_vrcharacter (cast `/Game/LSH_WorkSpace/BP_VRCharacter` (`GameplayStatics.GetPlayerCharacter` 0)))
  (add `/Game/LSH_WorkSpace/BP_VRCharacter.createdirty` _asbp_vrcharacter (delegate `createdirty_Event`)))

(event `build`)

(event `self.SM_BoxTruck_01a.OnComponentEndOverlap`
  (params (OverlappedComponent :type "PrimitiveComponent Object Reference") (OtherActor :type "Actor Object Reference") (OtherComp :type "PrimitiveComponent Object Reference") (OtherBodyIndex :type Integer)))

(event `move`)

(event `self.SM_BoxTruck_01a.OnComponentBeginOverlap`
  (params (OverlappedComponent :type "PrimitiveComponent Object Reference") (OtherActor :type "Actor Object Reference") (OtherComp :type "PrimitiveComponent Object Reference") (OtherBodyIndex :type Integer) (bFromSweep :type Boolean) (SweepResult :type "HitResult Structure (by ref)")))

(fn `UserConstructionScript`)