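; VR character Blueprint that paints red decals onto surfaces and wears them away while the left mouse button is held.
; Each tick it line-traces from the camera; in painting mode it attaches a decal at the hit and stores it.
; Key 1 turns painting off, so the trace instead steps nearby stored decals through successive material instances, matched by display name, then hides them.
; The drawing and painting flags live on a decal component.
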(event `Key|LeftMouseButton`
  (params (Key :type "Key Structure"))
  (bind _decalcompoenent (`self.DecalCompoenent`))
  (:`Pressed`
    (set `DecalCompoenent.IsDrawing` true _decalcompoenent))
  (:`Released`
    (set `DecalCompoenent.IsDrawing` false _decalcompoenent)))

(event `Key|One`
  (params (Key :type "Key Structure"))
  (:`Pressed`
    (set `DecalCompoenent.IsPainting` false (`self.DecalCompoenent`))))

(event `self.ReceiveTick`
  (params (DeltaSeconds :type "Float (single-precision)"))
  (bind _decal_comps (`self.Decal Comps`))
  (bind _transformcomponent (`PlayerCameraManager.TransformComponent` (`GameplayStatics.GetPlayerCameraManager` 0)))
  (bind _returnvalue (`SceneComponent.K2_GetComponentLocation` _transformcomponent))
  (if (`DecalCompoenent.IsDrawing` (`self.DecalCompoenent`))
    (bind (_outhit _returnvalue_2) (`KismetSystemLibrary.LineTraceSingle` :`Start` _returnvalue :`End` (+ _returnvalue (* (`SceneComponent.GetForwardVector` _transformcomponent) 10000.0)) :`TraceChannel` "TraceTypeQuery1" :`bTraceComplex` true :`DrawDebugType` "ForOneFrame"))
    (if _returnvalue_2
      (if (`DecalCompoenent.IsPainting` (`self.DecalCompoenent`))
        (bind (_bblockinghit _binitialoverlap _time _distance _location _impactpoint _normal _impactnormal _physmat _hitactor _hitcomponent) (`GameplayStatics.BreakHitResult` _outhit))
        (bind _returnvalue_3 (`GameplayStatics.SpawnDecalAttached` "/Game/LMH/Decal2/MI_RedDecal_1.MI_RedDecal_1" (2.0 2.0 2.0) _hitcomponent "None" _impactpoint (`KismetMathLibrary.Conv_VectorToRotator` _normal) "KeepWorldPosition"))
        (`KismetArrayLibrary.Array_Add` (`self.Decal Comps`) _returnvalue_3)
        (`DecalComponent.SetFadeScreenSize` _returnvalue_3 0.0)
        (set `self.IsCanDraw` true)
        (else
          (`/Engine/EditorBlueprintResources/StandardMacros.IsValid` (`|GetArrayItem` _decal_comps)
            (:`Is Valid`
              (for _array_element _decal_comps
                (if (< (`KismetMathLibrary.Vector_Distance` _location (`SceneComponent.K2_GetComponentLocation` _array_element)) 2.0)
                  (bind _returnvalue_4 (`KismetSystemLibrary.GetDisplayName` (`DecalComponent.GetDecalMaterial` _array_element)))
                  (`KismetSystemLibrary.PrintString` _returnvalue_4)
                  (switch `string` _returnvalue_4
                    (:`Default`
                      (`SceneComponent.SetHiddenInGame` _array_element true false))
                    (:`MI_RedDecal_1`
                      (`DecalComponent.SetDecalMaterial` _array_element "/Game/LMH/Decal2/MI_RedDecal_2.MI_RedDecal_2"))
                    (:`MI_RedDecal_2`
                      (`DecalComponent.SetDecalMaterial` _array_element "/Game/LMH/Decal2/MI_RedDecal_3.MI_RedDecal_3"))
                    (:`MI_RedDecal_3`
                      (`DecalComponent.SetDecalMaterial` _array_element "/Game/LMH/Decal2/MI_RedDecal_4.MI_RedDecal_4"))
                    (:`MI_RedDecal_4`
                      (`DecalComponent.SetDecalMaterial` _array_element "/Game/LMH/Decal2/MI_RedDecal_5.MI_RedDecal_5"))))))))))))

(event `self.ReceiveBeginPlay`)

(fn `UserConstructionScript`)