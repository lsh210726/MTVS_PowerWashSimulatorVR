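; BP_DrawActor paints brush marks into the RT_ClearBoard render target at requested 2D locations.
; On BeginPlay it stores all DecalActors, creates a dynamic WaterBrush material instance and calls a render target clear to black.
; Draw prints the location, sets it as the brush's DrawLocation parameter, then draws that material into the render target.
; The stored DecalActors are not used in this graph.
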(event `self.ReceiveBeginPlay`
  (`|ExecutionSequence`
    (:`then_0`
      (bind _outactors (`GameplayStatics.GetAllActorsOfClass` "/Script/Engine.DecalActor"))
      (set `self.Decal Actors` _outactors)
      (set `self.ClearBoard` "/Game/LMH/Decal/RT_ClearBoard.RT_ClearBoard")
      (bind _returnvalue (`KismetMaterialLibrary.CreateDynamicMaterialInstance` "/Game/LMH/Decal/WaterBrush.WaterBrush"))
      (set `self.WaterBrushMI` _returnvalue))
    (:`then_1`
      (`KismetRenderingLibrary.ClearRenderTarget2D` null))))

(event `/Game/LMH/Decal/BPI_DrawOnBoard.Draw`
  (params (`Location to Draw` :type "Vector2D Structure"))
  (bind _waterbrushmi (`self.WaterBrushMI`))
  (bind _clearboard (`self.ClearBoard`))
  (`KismetSystemLibrary.PrintString` (`KismetStringLibrary.Conv_Vector2dToString` `Location to Draw`))
  (`/Engine/EditorBlueprintResources/StandardMacros.IsValid` _waterbrushmi
    (:`Is Valid`
      (`MaterialInstanceDynamic.SetVectorParameterValue` _waterbrushmi "DrawLocation" (`KismetMathLibrary.Conv_VectorToLinearColor` (`KismetMathLibrary.Conv_Vector2DToVector` `Location to Draw` 0.1)))
      ;[1 1 1] target 에 mat그림
      (`/Engine/EditorBlueprintResources/StandardMacros.IsValid` _clearboard
        (:`Is Valid`
          (`KismetRenderingLibrary.DrawMaterialToRenderTarget` _clearboard _waterbrushmi))))))

(fn `UserConstructionScript`)