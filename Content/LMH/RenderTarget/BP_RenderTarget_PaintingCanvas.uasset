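; A paintable canvas actor that lets the player paint on its static mesh by aiming the camera and holding left mouse, with a debug sphere marking the brush.
; Each tick, a camera ray against the mesh finds the hit UV, which is passed with delta time to a dynamic brush material.
; The material draws into a render target copy created at BeginPlay, which is copied into the main target the material samples, forming a ping-pong accumulation.
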(event `self.ReceiveTick`
  (params (DeltaSeconds :type "Float (single-precision)"))
  (bind _brushmaterialinstance (`self.BrushMaterialInstance`))
  (bind _returnvalue (`PlayerController.IsInputKeyDown` (`GameplayStatics.GetPlayerController` 0) "LeftMouseButton"))
  (bind _transformcomponent (`PlayerCameraManager.TransformComponent` (`GameplayStatics.GetPlayerCameraManager` 0)))
  (bind _returnvalue_2 (`SceneComponent.K2_GetComponentLocation` _transformcomponent))
  (`|ExecutionSequence`
    (:`then_0`
      ;[1 1 1] Copy the temporary( writable) texture to the main one
      (bind (_canvas _size _context) (`KismetRenderingLibrary.BeginDrawCanvasToRenderTarget` (`self.PaintingRenderTarget`)))
      (`Canvas.K2_DrawTexture` _canvas (`self.PaintingRenderTargetCopy`) (0.0 0.0) _size (0.0 0.0) (1.0 1.0) (struct :`R` 1.0 :`G` 1.0 :`B` 1.0 :`A` 1.0) "BLEND_Opaque" 0.0 (0.5 0.5))
      (`KismetRenderingLibrary.EndDrawCanvasToRenderTarget` _context))
    (:`then_1`
      ;[1 1 1] Find world position for 3d brush on a surface of the painted object
      (bind (_hitlocation _hitnormal _bonename _outhit _returnvalue_3) (`PrimitiveComponent.K2_LineTraceComponent` (`self.StaticMesh`) _returnvalue_2 (+ _returnvalue_2 (* (`SceneComponent.GetForwardVector` _transformcomponent) 10000.0)) true false false))
      (if _returnvalue_3
        (`KismetSystemLibrary.DrawDebugSphere` _hitlocation 30.0 12 (`KismetMathLibrary.SelectColor` (struct :`R` 1.0 :`G` 0.847106 :`A` 1.0) (struct :`R` 1.0 :`G` 1.0 :`B` 1.0 :`A` 1.0) _returnvalue) 0.06 1.0)
        (bind (_uv _returnvalue_4) (`GameplayStatics.FindCollisionUV` _outhit))
        ;[1 1 1] Pass UVs of the hit to the material, pass
        (`MaterialInstanceDynamic.SetVectorParameterValue` _brushmaterialinstance "BrushPositionUV" (make `LinearColor` (`KismetMathLibrary.BreakVector2D` _uv) (`.Y` (`KismetMathLibrary.BreakVector2D` _uv)) (select `bool` (and _returnvalue_4 _returnvalue_3 _returnvalue) :`true` 1.0 :!type "Float (single-precision)") 1.0))
        (`MaterialInstanceDynamic.SetScalarParameterValue` _brushmaterialinstance "DeltaTime" (`GameplayStatics.GetWorldDeltaSeconds`))
        ;[1 1 1] Draw brush
        (bind (_canvas_2 _size_2 _context_2) (`KismetRenderingLibrary.BeginDrawCanvasToRenderTarget` (`self.PaintingRenderTargetCopy`)))
        (`Canvas.K2_DrawMaterial` _canvas_2 (`self.BrushMaterialInstance`) (0.0 0.0) _size_2 (0.0 0.0) (1.0 1.0) 0.0 (0.5 0.5))
        (`KismetRenderingLibrary.EndDrawCanvasToRenderTarget` _context_2)))))

(event `self.ReceiveBeginPlay`
  (bind _paintingrendertarget (`self.PaintingRenderTarget`))
  (bind _paintingrendertarget_2 (`self.PaintingRenderTarget`))
  (`|ExecutionSequence`
    (:`then_0`
      (`KismetRenderingLibrary.ClearRenderTarget2D` _paintingrendertarget (`TextureRenderTarget2D.ClearColor` _paintingrendertarget)))
    (:`then_1`
      (bind _returnvalue (`KismetMaterialLibrary.CreateDynamicMaterialInstance` (`self.BrushMaterialTemplate`) "MI_Brush"))
      (bind _output_get (set `self.BrushMaterialInstance` _returnvalue))
      (`MaterialInstanceDynamic.SetTextureParameterValue` _output_get "RenderTarget" (`self.PaintingRenderTarget`)))
    (:`then_2`
      (bind _returnvalue_2 (`KismetRenderingLibrary.CreateRenderTarget2D` (`TextureRenderTarget2D.SizeX` _paintingrendertarget_2) (`TextureRenderTarget2D.SizeY` _paintingrendertarget_2) (`TextureRenderTarget2D.RenderTargetFormat` _paintingrendertarget_2) (`TextureRenderTarget2D.ClearColor` _paintingrendertarget_2) (`TextureRenderTarget2D.bAutoGenerateMips` _paintingrendertarget_2)))
      (set `self.PaintingRenderTargetCopy` _returnvalue_2))))

(fn `UserConstructionScript`)