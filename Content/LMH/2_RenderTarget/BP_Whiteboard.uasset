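; Whiteboard actor that players draw on by painting a marker material into a render target.
; BeginPlay creates the dynamic marker, clears both boards' render targets and binds to the first-person character's brush and board change dispatchers.
; Draw events set the marker's location and size parameters; board change swaps the mesh material and switches to the second target.
; The brush change handler is empty, and the second-marker setup is disconnected.
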(event `BoardChange_Event`
  (`KismetSystemLibrary.PrintString` "222222222222" true true (struct :`R` 0.043377 :`B` 1.0 :`A` 1.0))
  (`PrimitiveComponent.SetMaterial` (`self.StaticMesh`) 0 "/Game/LMH/2_RenderTarget/3WhiteBoard.3WhiteBoard")
  (set `self.PaintBoard` "/Game/LMH/2_RenderTarget/2PaintBoard.2PaintBoard"))

(event `self.ReceiveBeginPlay`
  (`|ExecutionSequence`
    (:`then_0`
      (bind _returnvalue (`KismetMaterialLibrary.CreateDynamicMaterialInstance` "/Game/LMH/2_RenderTarget/WhiteBoardMarker.WhiteBoardMarker"))
      (set `self.WhiteBoardMarker` _returnvalue)
      (`KismetRenderingLibrary.ClearRenderTarget2D` (`self.PaintBoard`))
      (`KismetRenderingLibrary.ClearRenderTarget2D` "/Game/LMH/2_RenderTarget/2PaintBoard.2PaintBoard"))
    (:`then_1`
      (bind _asbp_lmhfirst_person_character (cast `/Game/LMH/2_RenderTarget/BP_LMHFirstPersonCharacter` (`GameplayStatics.GetPlayerCharacter` 0)))
      (add `/Game/LMH/2_RenderTarget/BP_LMHFirstPersonCharacter.BrushChange` _asbp_lmhfirst_person_character (delegate `BrushChange_Event`))
      (add `/Game/LMH/2_RenderTarget/BP_LMHFirstPersonCharacter.BoardChange` _asbp_lmhfirst_person_character (delegate `BoardChange_Event`))
      (set `self.PaintBoard` "/Game/LMH/2_RenderTarget/PaintBoard.PaintBoard"))))

(event `BrushChange_Event`)

(event `DrawOnWhiteBoard`
  (params (`Location to Draw` :type "Vector2D Structure"))
  (bind _whiteboardmarker (`self.WhiteBoardMarker`))
  (bind _whiteboardmarker2 (`self.WhiteBoardMarker2`))
  (if (`self.isTwo`)
    (`MaterialInstanceDynamic.SetVectorParameterValue` _whiteboardmarker2 "DrawLocation" (`KismetMathLibrary.Conv_VectorToLinearColor` (`KismetMathLibrary.Conv_Vector2DToVector` `Location to Draw` 0.1)))
    (`KismetRenderingLibrary.DrawMaterialToRenderTarget` (`self.PaintBoard`) _whiteboardmarker2)
    (else
      (`MaterialInstanceDynamic.SetVectorParameterValue` _whiteboardmarker "DrawLocation" (`KismetMathLibrary.Conv_VectorToLinearColor` (`KismetMathLibrary.Conv_Vector2DToVector` `Location to Draw` 0.1)))
      ;[1 1 1] target 에 mat그림
      (`KismetRenderingLibrary.DrawMaterialToRenderTarget` (`self.PaintBoard`) _whiteboardmarker))))

(event `DrawSize`
  (params (`Draw Size` :type "Float (double-precision)"))
  (`MaterialInstanceDynamic.SetScalarParameterValue` (`self.WhiteBoardMarker`) "Size" `Draw Size`))

(fn `UserConstructionScript`)