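; VR player character with a desktop mode, driving a building system and a decal painting component.
; Tab or left Y toggles the build menu as a 3D or viewport widget per IsVR, canceling placement on close; Click calls Move while it is open.
; Left click and right B feed widget interaction presses.
; Number keys control paint state, color and erase mode, while debug keys toggle IsVR and a spawned water gun.
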(event Input|EnhancedActionEvents|EnhancedInputActionIA_RightBBtn
  (params (ActionValue :type Boolean) (ElapsedSeconds :type Float%20%28double-precision%29) (TriggeredSeconds :type Float%20%28double-precision%29) (InputAction :type Input%20Action%20Object%20Reference :default "/Game/LSH_WorkSpace/Inputs/IA_RightBBtn.IA_RightBBtn")))

(event Input|EnhancedActionEvents|EnhancedInputActionIA_LeftYBtn
  (params (ActionValue :type Boolean) (ElapsedSeconds :type Float%20%28double-precision%29) (TriggeredSeconds :type Float%20%28double-precision%29) (InputAction :type Input%20Action%20Object%20Reference :default "/Game/LSH_WorkSpace/Inputs/IA_LeftYBtn.IA_LeftYBtn"))
  (bind _acbp_buildingsystem (Variables|Default|GetACBP_BuildingSystem))
  (:Triggered
    (Utilities|FlowControl|FlipFlop
      (:A
        (Variables|Default|Settabon true)
        (Variables|/Game/Dev/JJH/ACBP_BuildingSystem.ACBP_BuildingSystem_C|Setmeshclass (Variables|Default|GetACBP_BuildingSystem) 0)
        (Variables|/Script/Engine.PlayerController|SetbShowMouseCursor (Game|GetPlayerController 0) true)
        (if (Variables|Default|GetisVR)
          (Rendering|SetVisibility (Variables|Default|GetVRWidget) true false)
          (else
            (Widget|SetVisibility (Variables|Default|GetWB_Widget) "Visible"))))
      (:B
        (Variables|Default|Settabon false)
        (Variables|/Script/Engine.PlayerController|SetbShowMouseCursor (Game|GetPlayerController 0) false)
        (if (Variables|Default|GetisVR)
          (Rendering|SetVisibility (Variables|Default|GetVRWidget) false false)
          (Default|Cancle _acbp_buildingsystem)
          (else
            (Widget|SetVisibility (Variables|Default|GetWB_Widget) "Hidden")
            (Default|Cancle _acbp_buildingsystem)))))))

(event Input|EnhancedActionEvents|EnhancedInputActionIA_RightBBtn
  (params (ActionValue :type Boolean) (ElapsedSeconds :type Float%20%28double-precision%29) (TriggeredSeconds :type Float%20%28double-precision%29) (InputAction :type Input%20Action%20Object%20Reference :default "/Game/LSH_WorkSpace/Inputs/IA_RightBBtn.IA_RightBBtn"))
  (bind _widgetinteraction (Variables|Default|GetWidgetInteraction))
  (:Triggered
    (Class|WidgetInteractionComponent|PressPointerKey _widgetinteraction "LeftMouseButton"))
  (:Completed
    (Class|WidgetInteractionComponent|ReleasePointerKey _widgetinteraction "LeftMouseButton")))

(event EventBeginPlay
  (bind _returnvalue (UserInterface|CreateWidget "/Game/Dev/JJH/WB_BuildSystemWidget.WB_BuildSystemWidget_C"))
  (bind _output_get (Variables|Default|SetWB_Widget _returnvalue))
  (UserInterface|Viewport|AddtoViewport _output_get 0)
  (Widget|SetVisibility _output_get "Hidden")
  (bind _returnvalue_2 (Actor|GetActorOfClass "/Game/Dev/JJH/BP_Car.BP_Car_C"))
  (Variables|Default|Setcar1 _returnvalue_2)
  (Variables|Default|SetLeft%20Motion%20Controller (Variables|Default|GetleftMotionController)))

(event Collision|EventActorBeginOverlap
  (params (OtherActor :type Actor%20Object%20Reference)))

(event EventTick
  (params (DeltaSeconds :type Float%20%28single-precision%29)))

(event Input|ActionEvents|InputActionTabkey
  (params (Key :type Key%20Structure :default "None"))
  (bind _acbp_buildingsystem (Variables|Default|GetACBP_BuildingSystem))
  (:Pressed
    (Utilities|FlowControl|FlipFlop
      (:A
        (Variables|Default|Settabon true)
        (Variables|/Game/Dev/JJH/ACBP_BuildingSystem.ACBP_BuildingSystem_C|Setmeshclass (Variables|Default|GetACBP_BuildingSystem) 0)
        (Variables|/Script/Engine.PlayerController|SetbShowMouseCursor (Game|GetPlayerController 0) true)
        (if (Variables|Default|GetisVR)
          (Rendering|SetVisibility (Variables|Default|GetVRWidget) true false)
          (else
            (Widget|SetVisibility (Variables|Default|GetWB_Widget) "Visible"))))
      (:B
        (Variables|Default|Settabon false)
        (Variables|/Script/Engine.PlayerController|SetbShowMouseCursor (Game|GetPlayerController 0) false)
        (if (Variables|Default|GetisVR)
          (Rendering|SetVisibility (Variables|Default|GetVRWidget) false false)
          (Default|Cancle _acbp_buildingsystem)
          (else
            (Widget|SetVisibility (Variables|Default|GetWB_Widget) "Hidden")
            (Default|Cancle _acbp_buildingsystem)))))))

(event Input|ActionEvents|InputActionClick
  (params (Key :type Key%20Structure :default "None"))
  (:Pressed
    (if (Variables|Default|Gettabon)
      (Default|Move (Variables|Default|GetACBP_BuildingSystem)))))

(event Input|ActionEvents|InputActionLEFTCLICK
  (params (Key :type Key%20Structure :default "None"))
  (bind _widgetinteraction (Variables|Default|GetWidgetInteraction))
  (:Pressed
    (Class|WidgetInteractionComponent|PressPointerKey _widgetinteraction "LeftMouseButton"))
  (:Released
    (Class|WidgetInteractionComponent|ReleasePointerKey _widgetinteraction "LeftMouseButton")))

(event Input|KeyboardEvents|DebugKey5
  (params (Key :type Key%20Structure :default "None") (ActionValue :type Input%20Action%20Value%20Structure))
  (:Pressed
    (Utilities|FlowControl|FlipFlop
      (:A
        (bind _returnvalue (Game|SpawnActorfromClass "/Game/LSH_WorkSpace/BP_WaterGunActor.BP_WaterGunActor_C" (Transformation|GetActorTransform) "Undefined" "MultiplyWithRoot" 0 0)))
      (:B
        (Actor|DestroyActor _returnvalue)))))

(event Input|KeyboardEvents|DebugKey4
  (params (Key :type Key%20Structure :default "None") (ActionValue :type Input%20Action%20Value%20Structure))
  (:Pressed
    (Utilities|FlowControl|FlipFlop
      (:A
        (Variables|Default|SetisVR true))
      (:B
        (Variables|Default|SetisVR false)))))

(event Input|KeyboardEvents|1
  (params (Key :type Key%20Structure :default "None"))
  (bind _decalcomp (Variables|Default|GetdecalComp))
  (:Pressed
    (Utilities|FlowControl|FlipFlop
      (:A
        (Variables|/Script/PowerWash.DecalCompoenent|SetIsPainting _decalcomp false)
        (Variables|/Script/PowerWash.DecalCompoenent|SetPaintedTotalArea _decalcomp (Variables|/Script/PowerWash.DecalCompoenent|GetPaintedArea _decalcomp)))
      (:B
        (Variables|/Script/PowerWash.DecalCompoenent|SetIsPainting _decalcomp true)))))

(event Input|KeyboardEvents|2
  (params (Key :type Key%20Structure :default "None"))
  (bind _decalcomp (Variables|Default|GetdecalComp))
  (:Pressed
    (switch Utilities|FlowControl|Switch|SwitchonEPaintColor (Variables|/Script/PowerWash.DecalCompoenent|GetColor (Variables|Default|GetdecalComp))
      (:Red
        (Variables|/Script/PowerWash.DecalCompoenent|SetColor _decalcomp "Yellow"))
      (:Yellow
        (Variables|/Script/PowerWash.DecalCompoenent|SetColor _decalcomp "Green"))
      (:Green
        (Variables|/Script/PowerWash.DecalCompoenent|SetColor _decalcomp "Red")))))

(event Input|KeyboardEvents|3
  (params (Key :type Key%20Structure :default "None"))
  (bind _decalcomp (Variables|Default|GetdecalComp))
  (:Pressed
    (switch Utilities|FlowControl|Switch|SwitchonEEraseMode (Variables|/Script/PowerWash.DecalCompoenent|GeteraseMode _decalcomp)
      (:AllClear
        (Variables|/Script/PowerWash.DecalCompoenent|SeteraseMode _decalcomp "FourStatge"))
      (:FourStatge
        (Variables|/Script/PowerWash.DecalCompoenent|SeteraseMode _decalcomp "AllClear")))))

(fn ConstructionScript)